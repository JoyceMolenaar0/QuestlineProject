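; Base quest actor that tracks objective progress for the current stage of a quest and notifies the player on completion.
; On BeginPlay it loads quest details by QuestID from a data table, zeroes a per-objective progress map and binds to the player character's OnObjectiveIDCalled event.
; OnObjectiveIDHeard increments matching objectives up to their required quantity, then IsObjectiveComplete shows a notification widget for finished ones.
; No stage advancement is implemented here.
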(event EventBeginPlay
  (CallFunction|GetQuestDetails)
  (EventDispatchers|BindEventtoOnObjectiveIDCalled (CallFunction|GetMyPlayerCharacter) (EventDispatchers|CreateEvent :!event OnObjectiveIDHeard)))

(event Collision|EventActorBeginOverlap
  (params (OtherActor :type Actor%20Object%20Reference)))

(event EventTick
  (params (DeltaSeconds :type Float%20%28single-precision%29)))

(fn ConstructionScript)

(fn OnObjectiveIDHeard
  (params (ObjectiveID :type String))
  (bind _currentobjectiveprogress (Variables|Default|GetCurrentObjectiveProgress))
  (bind (_value _returnvalue) (Utilities|Map|Find _currentobjectiveprogress ObjectiveID))
  (if _returnvalue
    (if (< _value (Utilities|Struct|BreakSTRUCT_ObjectiveDetails (CallFunction|GetObjectiveDatabyID ObjectiveID)))
      (Utilities|Map|Add (Variables|Default|GetCurrentObjectiveProgress) ObjectiveID (+ _value 1))
      (CallFunction|IsObjectiveComplete ObjectiveID)
      (return))
    (else
      (return))))

(fn GetQuestDetails
  (bind _returnvalue (Utilities|GetDataTableRow "/Game/QuestSystem/Data/Data_QuestData.Data_QuestData" (Variables|Default|GetQuestID))
    (:then
      (bind _output_get (Variables|Default|SetQuestDetails _returnvalue))
      (bind _output_get_2 (Variables|Default|SetCurrentStageDetails (Utilities|Array|Get(acopy) (Utilities|Struct|BreakSTRUCT_QuestDetails _output_get) (Variables|Default|GetCurrentStage))))
      (Utilities|Map|Clear (Variables|Default|GetCurrentObjectiveProgress))
      (for _array_element (Utilities|Struct|BreakSTRUCT_StageDetails _output_get_2)
        (Utilities|Map|Add (Variables|Default|GetCurrentObjectiveProgress) (Utilities|Struct|BreakSTRUCT_ObjectiveDetails _array_element) 0)))))

(fn GetObjectiveDatabyID
  (params (ObjecitveID :type String))
  (for _array_element (Utilities|Struct|BreakSTRUCT_StageDetails (Variables|Default|GetCurrentStageDetails))
    (if (Utilities|Enum|Equal(Enum) (Utilities|Struct|BreakSTRUCT_ObjectiveDetails _array_element) ObjecitveID)
      (return _array_element))))

(fn IsObjectiveComplete
  (params (ObjectiveID :type String))
  (bind _array_element (CallFunction|GetObjectiveDatabyID ObjectiveID))
  (bind (_description _quantity) (Utilities|Struct|BreakSTRUCT_ObjectiveDetails _array_element))
  (if (>= (.Value (Utilities|Map|Find (Variables|Default|GetCurrentObjectiveProgress) ObjectiveID)) _quantity)
    (bind _returnvalue (UserInterface|CreateWidget "/Game/QuestSystem/UI/QuestNotify/W_QuestNotifiaction.W_QuestNotifiaction_C" 0 _description))
    (UserInterface|Viewport|AddtoViewport _returnvalue 0)
    (else
      (Development|PrintString "False"))))